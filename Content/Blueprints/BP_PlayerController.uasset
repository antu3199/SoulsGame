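; BP_PlayerController is a player controller that handles camera-relative movement and look input for the controlled pawn.
; Each Tick it feeds the MoveForward and MoveRight axis values into the pawn's movement input along the camera's forward and right vectors.
; The forward vector comes from the full camera rotation, so it includes pitch.
; RotateCamera and ChangePitch axis events drive controller yaw and pitch.
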(event EventBeginPlay)

(event EventTick
  (params (DeltaSeconds :type Float%20%28single-precision%29))
  (bind _returnvalue (Pawn|GetControlledPawn))
  (bind _playercameramanager (Variables|Default|GetPlayerCameraManager))
  (bind _returnvalue_2 (Camera|GetCameraRotation _playercameramanager))
  ;[1 1 1] Movement
  (Pawn|Input|AddMovementInput _returnvalue (Math|Vector|GetForwardVector _returnvalue_2) (Input|AxisValues|GetMoveForward) false)
  (Pawn|Input|AddMovementInput _returnvalue (Math|Vector|GetRightVector _returnvalue_2) (Input|AxisValues|GetMoveRight) false))

(event Input|AxisEvents|InputAxisRotateCamera
  (params (AxisValue :type Float%20%28single-precision%29))
  ;[1 1 1] Camera rotation
  (Class|PlayerController|AddYawInput AxisValue))

(event Input|AxisEvents|InputAxisChangePitch
  (params (AxisValue :type Float%20%28single-precision%29))
  ;[1 1 1] Camera rotation
  (Class|PlayerController|AddPitchInput AxisValue))

(fn ConstructionScript)